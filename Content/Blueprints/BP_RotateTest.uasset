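; Prototype player actor that orbits a BP_Planet, dives through it and kills slower players on overlap to score.
; Horizontal input rotates its position around the planet axis; Dive moves it straight across until back at grounded radius, launching into decaying flight if the trigger is held, then sinking back.
; Speed from these motions decides hits and drives color brightness and movement volume.
; Victims lose collision until a respawn timer expires.
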(event EventBeginPlay
  (if (== (Variables|Default|GetTarget) 0)
    (bind _outactors (Actor|GetAllActorsOfClass "/Game/Blueprints/BP_Planet.BP_Planet_C"))
    (bind _output_get (Variables|Default|SetTarget (Utilities|Array|Get(acopy) _outactors)))
    (Variables|Default|SetGroundedDistance (Transformation|GetDistanceTo _output_get))))

(event Collision|EventActorBeginOverlap
  (params (OtherActor :type Actor%20Object%20Reference))
  (if (not (== OtherActor (Variables|Default|GetTarget)))
    (bind _asbp_rotate_test (Utilities|Casting|CastToBP_RotateTest OtherActor))
    (if (< (Variables|BP_RotateTest_C|GetSpeedValue _asbp_rotate_test) (Variables|Default|GetSpeedValue))
      (Variables|BP_RotateTest_C|SetDead _asbp_rotate_test true)
      (Variables|BP_RotateTest_C|SetRespawnTimer _asbp_rotate_test (Variables|Default|GetRespawnTime))
      (Collision|SetCollisionEnabled (Variables|BP_RotateTest_C|GetSphere _asbp_rotate_test) "NoCollision")
      (Audio|Components|Audio|Play (Variables|Default|GetSE_Hit) 0.0)
      (Math|Integer|IncrementInt (Variables|Default|GetScore)))))

(event EventTick
  (params (DeltaSeconds :type Float%20%28single-precision%29))
  (bind _originalcolor (Variables|Default|GetOriginalColor))
  (bind (_x _y _z) (Math|Vector|BreakVector _originalcolor))
  (if (Variables|Default|GetDead)
    (Variables|Default|SetSpeedValue -35.0)
    (bind _output_get (Variables|Default|SetRespawnTimer (- (Variables|Default|GetRespawnTimer) DeltaSeconds)))
    (if (< _output_get 0.0)
      (Variables|Default|SetDead false)
      (Collision|SetCollisionEnabled (Variables|Default|GetSphere) "QueryAndPhysics"))
    (else
      (Variables|Default|SetSpeedValue (+ (Math|Float|Absolute(Float) (Math|Vector|VectorLength (Variables|Default|GetDiveVector))) (Math|Float|Absolute(Float) (* (Variables|Default|GetCurrentSpeed) (Variables|Default|GetSpeedBias))) (Math|Float|Absolute(Float) (* (Variables|Default|GetFlightAddition) (Variables|Default|GetFlightBias)))))))
  (bind _returnvalue (Rendering|Material|CreateDynamicMaterialInstance (Variables|Default|GetStaticMesh) 0 0 "None" :!class /Script/Engine.PrimitiveComponent))
  (Rendering|Material|SetVectorParameterValue _returnvalue "Color" (Math|Color|MakeColor (+ _x (/ (Variables|Default|GetSpeedValue) (Variables|Default|GetMaxSpeed))) (+ _y (/ (Variables|Default|GetSpeedValue) (Variables|Default|GetMaxSpeed))) (+ _z (/ (Variables|Default|GetSpeedValue) (Variables|Default|GetMaxSpeed)))) :!class /Script/Engine.MaterialInstanceDynamic)
  (Audio|Components|Audio|SetVolumeMultiplier (Variables|Default|GetSE_Moving) (* (/ (Variables|Default|GetSpeedValue) (Variables|Default|GetMaxSpeed)) (Variables|Default|GetMovementSoundMultiplier)) :!class /Script/Engine.AudioComponent)
  (if (Variables|Default|GetDiving)
    (CallFunction|Dive)
    (elif (Variables|Default|GetFlying)
      (CallFunction|Fly)
      (elif (not (Variables|Default|GetGrounded))
        (Transformation|AddActorLocalOffset (* (Math|Vector|GetForwardVector (Math|Rotator|FindLookatRotation (Transformation|GetActorLocation) (Transformation|GetActorLocation (Variables|Default|GetTarget)))) 10) false false)
        (Variables|Default|SetGrounded (Math|Float|NearlyEqual(Float) (Variables|Default|GetGroundedDistance) (Transformation|GetDistanceTo (Variables|Default|GetTarget)) 1e+01))
        (else
          (Variables|Default|SetGrounded true))))))

(event Input|AxisEvents|InputAxisMoveHorizontal
  (params (AxisValue :type Float%20%28single-precision%29))
  (if (not (Variables|Default|GetDiving))
    (bind _output_get (Variables|Default|SetCurrentSpeed (Math|Interpolation|FInterpTo (stale _output_get) (* AxisValue (Variables|Default|GetRotateAmount)) (Utilities|Time|GetWorldDeltaSeconds) (Variables|Default|GetRotateSpeed))))
    (Transformation|SetActorLocation (Math|Vector|MakeVector 0.0 (.Y (Math|Vector|BreakVector (Math|Vector|RotateVectorAroundAxis (Transformation|GetActorLocation) _output_get (Transformation|GetActorForwardVector (Variables|Default|GetTarget))))) (.Z (Math|Vector|BreakVector (Math|Vector|RotateVectorAroundAxis (Transformation|GetActorLocation) _output_get (Transformation|GetActorForwardVector (Variables|Default|GetTarget)))))) false false)))

(event Input|AxisEvents|InputAxisDive
  (params (AxisValue :type Float%20%28single-precision%29))
  (Variables|Default|SetCurrentTriggerInput AxisValue)
  (if (Math|Boolean|ANDBoolean (> AxisValue 0.5) (not (Variables|Default|GetDiving)) (not (Variables|Default|GetFlying)) (Variables|Default|GetGrounded))
    (Variables|Default|SetCurrentSpeed 0.0)
    (Utilities|FlowControl|DoOnce false :!label _label
      (:Completed
        (Variables|Default|SetDiving true)
        (bind _output_get (Variables|Default|SetDiveVector (* (Math|Vector|GetForwardVector (Math|Rotator|FindLookatRotation (Transformation|GetActorLocation) (Transformation|GetActorLocation (Variables|Default|GetTarget)))) (* AxisValue (Variables|Default|GetDiveAmount)))))
        (Transformation|SetActorLocation (+ (Transformation|GetActorLocation) _output_get) false false)
        (Audio|Components|Audio|Play (Variables|Default|GetSE_Dive) 0.0)))
    (else
      (goto _label Reset))))

(fn ConstructionScript)

(fn MoveHorizontal
  (params (AxisValue :type Float%20%28single-precision%29)))

(fn Dive
  (Transformation|SetActorLocation (+ (Transformation|GetActorLocation) (Variables|Default|GetDiveVector)) false false)
  (if (Math|Float|NearlyEqual(Float) (Math|Float|Absolute(Float) (Transformation|GetDistanceTo (Variables|Default|GetTarget))) (Variables|Default|GetGroundedDistance) 25.0)
    (Variables|Default|SetDiving false)
    (Variables|Default|SetCurrentSpeed 0.0)
    (Variables|Default|SetDiveVector "0, 0, 0")
    (if (> (Variables|Default|GetCurrentTriggerInput) 0.5)
      (Variables|Default|SetFlying true)
      (Variables|Default|SetFlightAddition (Variables|Default|GetMaxHeight)))))

(fn Fly
  (Variables|Default|SetGrounded false)
  (Transformation|AddActorLocalOffset (* (Math|Vector|GetForwardVector (Math|Rotator|FindLookatRotation (Transformation|GetActorLocation) (Transformation|GetActorLocation (Variables|Default|GetTarget)))) (* (Variables|Default|GetFlightAddition) -1.0)) false false)
  (Variables|Default|SetFlightAddition (Math|Interpolation|FInterpTo (Variables|Default|GetFlightAddition) 0.0 (Utilities|Time|GetWorldDeltaSeconds) 1e+01))
  (if (Math|Float|NearlyEqual(Float) (Math|Interpolation|FInterpTo (Variables|Default|GetFlightAddition) 0.0 (Utilities|Time|GetWorldDeltaSeconds) 1e+01) 0.0 1.0)
    (Variables|Default|SetFlying false)
    (Variables|Default|SetGrounded false)))